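; AI controller for daily-life NPCs that runs Basic_BT and picks the actor to use for the chosen activity.
; On possess it maps level TargetPoints by name.
; While TargetActor is empty, perception updates match sensed beds or chairs to the blackboard's non-idle activity through UsableInterface_BP.
; IsSelfActivity returns true for those furniture activities despite its name; false makes the pawn target itself, and Conversation&Sit and Ping Pong remain unhandled.
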(event OnPerceptionUpdated(AIPerception)
  (params (UpdatedActors :type Array%20of%20Actor%20Object%20References))
  (for _array_element UpdatedActors
    (if (Utilities|DoesObjectImplementInterface (stale _array_element) "/Game/Blueprints/UsableInterface_BP.UsableInterface_BP_C")
      (bind _isusable (Class|UsableInterfaceBP|CanbeUsed(Message) (stale _array_element)))
      (if _isusable
        _))))

(event OnTargetPerceptionUpdated(AIPerception)
  (params (Actor :type Actor%20Object%20Reference) (Stimulus :type AI%20Stimulus%20Structure))
  (bind _returnvalue (AI|GetBlackboard 0))
  (bind _returnvalue_2 (AI|GetBlackboard 0))
  (bind _activitychosenkeyname (Variables|Default|GetActivityChosenKeyName))
  (bind _selfactorkeyname (Variables|Default|GetSelfActorKeyName))
  (bind _returnvalue_3 (Class|BlackboardComponent|GetValueasEnum _returnvalue _activitychosenkeyname))
  (bind _returnvalue_4 (AI|Components|Blackboard|GetValueasObject _returnvalue_2 _selfactorkeyname))
  (bind _returnvalue_5 (Utilities|Enum|ByteToEnumActivityState _returnvalue_3))
  (Utilities|IsValid (AI|Components|Blackboard|GetValueasObject (AI|GetBlackboard 0) (Variables|Default|GetTargetActorKeyName)) ; If Target Actor is NULL
    (:Is%20Not%20Valid
      (if (Utilities|Enum|NotEqual(Enum) _returnvalue_5 "NewEnumerator0") ; if the chosen activity is IDLE: do not care about sensing...
        (bind _istargetrequired (CallFunction|IsSelfActivity _returnvalue_5))
        (if _istargetrequired
          (switch Utilities|FlowControl|Switch|SwitchonActivityState _returnvalue_5
            (:NewEnumerator0
              (Development|PrintString "ERROR!" true true "(R=1.000000,G=0.019096,B=0.000000,A=1.000000)" :!label _label))
            (:NewEnumerator10
              (Utilities|Casting|CastToUsableBed Actor)
              (bind _isusable (Class|UsableInterfaceBP|CanbeUsed(Message) Actor :!label _label_2))
              (if (and _isusable (Utilities|DoesObjectImplementInterface Actor "/Game/Blueprints/UsableInterface_BP.UsableInterface_BP_C"))
                (AI|Components|Blackboard|SetValueasObject (AI|GetBlackboard 0) (Variables|Default|GetTargetActorKeyName) Actor)))
            (:NewEnumerator2
              (Utilities|Casting|CastToUsableChair Actor)
              (goto _label_2))
            (:NewEnumerator3
              (Utilities|Casting|CastToUsableChair Actor
                (:then
                  (goto _label_2))
                (:CastFailed
                  (Utilities|Casting|CastToUsableTableChair Actor :!label _label_3)
                  (goto _label_2))))
            (:NewEnumerator4
              (goto _label))
            (:NewEnumerator6
              (goto _label_3))
            (:NewEnumerator8
              (Utilities|Casting|CastToUsableGamingChair Actor)
              (goto _label_2))
            (:NewEnumerator1
              (goto _label))
            (:NewEnumerator5
              (goto _label))
            (:NewEnumerator9
              (Development|PrintString "DA GESTIRE!!!" true true "(R=1.000000,G=0.958813,B=0.000000,A=1.000000)" :!label _label_4))
            (:NewEnumerator7
              (goto _label_4)))
          (else
            (bind _isusable_2 (Class|UsableInterfaceBP|CanbeUsed(Message) _returnvalue_4)) ; If the activity is a lone activity and does not involve other actors: set SELF as TargetActor
            (if _isusable_2
              (AI|Components|Blackboard|SetValueasObject (AI|GetBlackboard 0) (Variables|Default|GetTargetActorKeyName) _returnvalue_4))))))))

(event EventTick
  (params (DeltaSeconds :type Float%20%28single-precision%29)))

(event EventPossess
  (params (PossessedPawn :type Pawn%20Object%20Reference))
  (AI|RunBehaviorTree "/Game/AI/Basic_BT.Basic_BT")
  (Variables|Default|SetAIState "NewEnumerator0")
  (bind _outactors (Actor|GetAllActorsOfClass "/Script/Engine.TargetPoint"))
  (for _array_element _outactors
    (Utilities|Map|Add (Variables|Default|GetTargetPointLocations) (Utilities|String|StringToName (Utilities|GetObjectName _array_element)) _array_element)))

(fn ConstructionScript)

(fn IsSitting
  (switch Utilities|FlowControl|Switch|SwitchonActivityState (Variables|Default|GetAIState)
    (:NewEnumerator0
      _)
    (:NewEnumerator2
      (return true))
    (:NewEnumerator3
      (return true))
    (:NewEnumerator4
      _)
    (:NewEnumerator6
      (return true))
    (:NewEnumerator8
      (return true))
    (:NewEnumerator1
      _)
    (:NewEnumerator5
      _)
    (:NewEnumerator9
      (return true))
    (:NewEnumerator7
      _))
  (return false))

(fn IsLoneActivity
  (params (Activity :type ActivityState%20Enum :default "NewEnumerator0"))
  (switch Utilities|FlowControl|Switch|SwitchonActivityState Activity
    (:NewEnumerator0
      _)
    (:NewEnumerator10
      _)
    (:NewEnumerator2
      _)
    (:NewEnumerator3
      _)
    (:NewEnumerator4
      _)
    (:NewEnumerator6
      _)
    (:NewEnumerator8
      _)
    (:NewEnumerator1
      (return false))
    (:NewEnumerator5
      (return false))
    (:NewEnumerator9
      (return false))
    (:NewEnumerator7
      (return false)))
  (return true))

(fn IsSelfActivity
  (params (Activity :type ActivityState%20Enum :default "NewEnumerator0"))
  (switch Utilities|FlowControl|Switch|SwitchonActivityState Activity
    (:NewEnumerator0
      _)
    (:NewEnumerator10
      (return true))
    (:NewEnumerator2
      (return true))
    (:NewEnumerator3
      (return true))
    (:NewEnumerator4
      _)
    (:NewEnumerator6
      (return true))
    (:NewEnumerator8
      (return true))
    (:NewEnumerator1
      _)
    (:NewEnumerator5
      _)
    (:NewEnumerator9
      (return true))
    (:NewEnumerator7
      (return true)))
  (return false))