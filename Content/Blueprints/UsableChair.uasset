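; UsableChair is a chair that one AI pawn at a time can occupy, for actors driven by AIControllerDailyLife_BP.
; Used marks it unavailable through the flag CanBeUsed returns, saves the controlled pawn's transform, then snaps the pawn onto the mesh's UseSocket.
; ResetUsage frees the chair, detaches the pawn and restores its saved transform.
; UseObject is empty, and some sitting height-offset logic is left unconnected.
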(event EventResetUsage
  (bind _usingpawnactor (Variables|Default|GetUsingPawnActor))
  (Variables|Default|SetIsUsable true)
  (Transformation|DetachFromActor _usingpawnactor "KeepRelative" "KeepRelative" "KeepRelative")
  (Transformation|SetActorTransform _usingpawnactor (Variables|Default|GetDeltaTransform)))

(event EventUseObject
  (params (UsedObject :type Actor%20Object%20Reference)))

(event EventUsed
  (params (UsingActor :type Actor%20Object%20Reference) (Value :type Integer))
  (Variables|Default|SetIsUsable false)
  (bind _asaicontroller_daily_life_bp (Utilities|Casting|CastToAIControllerDailyLife_BP UsingActor))
  (bind _output_get (Variables|Default|SetUsingPawnActor (Pawn|GetControlledPawn _asaicontroller_daily_life_bp)))
  (Variables|Default|SetDeltaTransform (Transformation|GetActorTransform _output_get))
  (Transformation|AttachComponentToComponent _output_get (Variables|Debug|GetStaticMeshComponent) "UseSocket" "SnapToTarget" "SnapToTarget" "SnapToTarget" false))

(fn ConstructionScript)

(fn CanbeUsed
  (params (UsingActor :type Actor%20Object%20Reference))
  (return (Variables|Default|GetIsUsable)))