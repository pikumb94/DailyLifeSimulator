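; Usable table that AI guys occupy through its child chair actors, with checks for solo use, group use and group joining.
; On use, it claims a free UsableTableChair and maps the user to it, so reset releases that same chair.
; An empty timer, randomized by the guy's LonePreference when the table is usable, supplies the duration written to the controller's BlackboardTime.
; CanBeUsed overwrites CurrentUsers with the free-chair count.
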(event Custom|CustomEvent_0)

(event EventResetUsage
  (params (ResetInvokerActor :type Actor%20Object%20Reference))
  (bind _usetable (Variables|Default|GetUseTable))
  (bind (_value _returnvalue) (Utilities|Map|Find _usetable ResetInvokerActor))
  (Variables|Default|SetCurrentUsers (- (Variables|Default|GetCurrentUsers) 1))
  (Variables|Default|SetIsUsable true)
  (Class|UsableInterfaceBP|ResetUsage(Message) _value) ; Propagate reset to the right child object
  (if _returnvalue
    (Utilities|Map|Remove _usetable ResetInvokerActor)
    (else
      (Development|PrintString "CHIDL NOT FOUND" true true "(R=1.000000,G=0.000000,B=0.000000,A=1.000000)"))))

(event EventUsed
  (params (UsingActor :type Actor%20Object%20Reference) (Value :type Integer))
  (Variables|Default|SetCurrentUsers (+ (Variables|Default|GetCurrentUsers) 1))
  (bind _asaicontroller_daily_life_bp (Utilities|Casting|CastToAIControllerDailyLife_BP UsingActor))
  (bind _asaiguy (Utilities|Casting|CastToAIGuy (Pawn|GetControlledPawn _asaicontroller_daily_life_bp)))
  (if (Variables|Default|GetIsUsable)
    (bind _returnvalue (Utilities|Time|SetTimerbyEvent (delegate Custom|CustomEvent_0) (+ (* (Math|Random|RandomFloatinRange (- 1.0 (Variables|/Game/Blueprints/AIGuy.AIGuy_C|GetLonePreference _asaiguy)) 1.0) 3e+01) 3e+01))))
  (Variables|Default|SetIsUsable false)
  (AI|Components|Blackboard|SetValueasFloat (AI|GetBlackboard _asaicontroller_daily_life_bp) (Utilities|Name|MakeLiteralName "BlackboardTime") (Utilities|Time|GetTimerRemainingTimebyHandle _returnvalue))
  (bind _usableobject (CallFunction|GetUsableObject))
  (Class|UsableInterfaceBP|Used(Message) _usableobject UsingActor) ; AIGuy use also the child object
  (Utilities|Map|Add (Variables|Default|GetUseTable) UsingActor _usableobject))

(fn ConstructionScript)

(fn GetUsableObject
  (for _array_element (Actor|GetAllChildActors true)
    (bind _asusable_table_chair (Utilities|Casting|CastToUsableTableChair _array_element))
    (bind _isusable (Class|UsableInterfaceBP|CanbeUsed(Message) _asusable_table_chair))
    (if _isusable
      (return _asusable_table_chair)))
  (return 0))

(fn CanbeGroupJoined
  (params (UsingActor :type Actor%20Object%20Reference))
  (bind _isusable (Class|UsableInterfaceBP|CanbeUsed(Message) self))
  (return (and _isusable (> (Utilities|Map|Length (Variables|Default|GetUseTable)) 0))))

(fn CanbeGroupUsed
  (params (UsingActor :type Actor%20Object%20Reference))
  (if (>= (Class|KismetMathLibrary|ToInt64(Integer) (- (Math|Conversions|ToInteger(Byte) (Variables|Default|GetMaxUsers)) (Math|Conversions|ToInteger(Byte) (Variables|Default|GetCurrentUsers)))) 2)
    (return true)
    (else
      (return false))))

(fn CanbeUsed
  (params (UsingActor :type Actor%20Object%20Reference))
  (for _array_element (Actor|GetAllChildActors true)
    (bind _asusable_table_chair (Utilities|Casting|CastToUsableTableChair _array_element))
    (bind _isusable (Class|UsableInterfaceBP|CanbeUsed(Message) _asusable_table_chair))
    (if _isusable
      (Math|Integer|IncrementInt (Math|Conversions|ToInteger(Byte) (LocalVariables|GetUsersCount)))))
  (Variables|Default|SetCurrentUsers (LocalVariables|GetUsersCount))
  (if (>= (Variables|Default|GetCurrentUsers) (Variables|Default|GetMaxUsers))
    (return false)
    (else
      (return true))))