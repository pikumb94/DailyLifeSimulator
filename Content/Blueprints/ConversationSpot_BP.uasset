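; Short-lived usable conversation spot for daily-life AI that relocates to a random navigable point around the NavMeshBoundsVolume on BeginPlay.
; Using it increments the user count, passes the remaining lifespan to the AI controller's BlackboardTime key, and updates availability against MaxUsers.
; ResetUsage decrements the count and destroys the spot once one or no users remain; otherwise it expires on its lifespan.
; Group use and joining are disabled.
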(event EventResetUsage
  (params (ResetInvokerActor :type Actor%20Object%20Reference))
  (bind _output_get (Variables|Default|SetCurrentUsers (- (Variables|Default|GetCurrentUsers) 1)))
  (if (<= _output_get 1)
    (Actor|DestroyActor)
    (else
      (bind _isusable (CallFunction|CanbeUsed))
      (Variables|Default|SetIsUsable _isusable))))

(event EventBeginPlay
  (bind _returnvalue (Actor|GetActorOfClass "/Script/NavigationSystem.NavMeshBoundsVolume"))
  (bind _randomlocation (Class|NavigationSystemV1|GetRandomLocationinNavigableRadius (.Origin (Collision|GetActorBounds _returnvalue false false)) (Math|Float|Max(Float) (.X (Math|Vector|BreakVector (.BoxExtent (Collision|GetActorBounds _returnvalue false false)))) (.Y (Math|Vector|BreakVector (.BoxExtent (Collision|GetActorBounds _returnvalue false false))))) 0 0))
  (Transformation|SetWorldLocation (Variables|Default|GetCapsule) _randomlocation false false)
  (Rendering|Debug|DrawDebugSphere (Transformation|GetActorLocation) 1e+02 12 "(R=0.000000,G=1.000000,B=0.000000,A=1.000000)" 5.0)
  (Actor|SetLifeSpan 15.0))

(event EventUsed
  (params (UsingActor :type Actor%20Object%20Reference) (Value :type Integer))
  (Variables|Default|SetCurrentUsers (+ (Variables|Default|GetCurrentUsers) 1))
  (bind _asaicontroller_daily_life_bp (Utilities|Casting|CastToAIControllerDailyLife_BP UsingActor))
  (AI|Components|Blackboard|SetValueasFloat (AI|GetBlackboard _asaicontroller_daily_life_bp) (Utilities|Name|MakeLiteralName "BlackboardTime") (Actor|GetLifeSpan))
  (bind _isusable (CallFunction|CanbeUsed))
  (Variables|Default|SetIsUsable _isusable))

(fn ConstructionScript)

(fn CanbeGroupJoined
  (params (UsingActor :type Actor%20Object%20Reference))
  (return false))

(fn CanbeGroupUsed
  (params (UsingActor :type Actor%20Object%20Reference))
  (return false))

(fn CanbeUsed
  (params (UsingActor :type Actor%20Object%20Reference))
  (if (>= (Variables|Default|GetCurrentUsers) (Variables|Default|GetMaxUsers))
    (return false)
    (else
      (return true))))