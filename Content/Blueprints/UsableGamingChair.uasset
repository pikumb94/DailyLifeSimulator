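; Usable gaming chair that one daily-life AI character at a time can occupy; group use and joining are disabled.
; On use it marks itself unavailable, saves the AI pawn's transform and snaps the pawn to the mesh's UseSocket.
; On reset it becomes usable again, detaches the pawn and restores the saved transform.
; Both events expect an AIControllerDailyLife_BP as the actor.
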(event EventResetUsage
  (params (ResetInvokerActor :type Actor%20Object%20Reference))
  (Variables|Default|SetIsUsable true)
  (bind _asaicontroller_daily_life_bp (Utilities|Casting|CastToAIControllerDailyLife_BP ResetInvokerActor))
  (Transformation|DetachFromActor (Pawn|GetControlledPawn _asaicontroller_daily_life_bp) "KeepRelative" "KeepRelative" "KeepWorld")
  (Transformation|SetActorTransform (Pawn|GetControlledPawn _asaicontroller_daily_life_bp) (Variables|Default|GetDeltaTransform)))

(event EventUsed
  (params (UsingActor :type Actor%20Object%20Reference) (Value :type Integer))
  (Variables|Default|SetIsUsable false)
  (bind _asaicontroller_daily_life_bp (Utilities|Casting|CastToAIControllerDailyLife_BP UsingActor))
  (Variables|Default|SetDeltaTransform (Transformation|GetActorTransform (Pawn|GetControlledPawn _asaicontroller_daily_life_bp)))
  (Transformation|AttachComponentToComponent (Pawn|GetControlledPawn _asaicontroller_daily_life_bp) (Variables|Debug|GetStaticMeshComponent) "UseSocket" "SnapToTarget" "SnapToTarget" "KeepWorld" false))

(fn ConstructionScript)

(fn CanbeGroupJoined
  (params (UsingActor :type Actor%20Object%20Reference))
  (return false))

(fn CanbeGroupUsed
  (params (UsingActor :type Actor%20Object%20Reference))
  (return false))

(fn CanbeUsed
  (params (UsingActor :type Actor%20Object%20Reference))
  (return (Variables|Default|GetIsUsable)))