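; AIGuy is an AI character in a daily-life simulation, tinted yellow, red or blue from its AIControllerDailyLife_BP type when possessed.
; It is also a usable object: Used adds to a displayed value and locks it, and ResetUsage unlocks it only if locked.
; When its own controller is the user, both apply or undo a sleeping-pose transform based on the Blackboard activity.
; UseObject is empty, and the attachment, animation and object-snapping chains are unwired.
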(event EventResetUsage
  ;[1 1 1] AIGuy Reset is IDEMPOTENT
  (if (not (Variables|Default|GetIsUsable))
    (Variables|Default|SetIsUsable true)
    (Rendering|Components|TextRender|SetText (Variables|Default|GetTextRender) (Utilities|Text|ToText(Integer) (- (Variables|Default|GetInnerValue) 1)))
    (if (== (stale EventUsed UsingActor) (AI|GetAIController self))
      (CallFunction|UpdateTransformforSelfActivity))))

(event EventPossessed
  (params (NewController :type Controller%20Object%20Reference))
  (bind _asaicontroller_daily_life_bp (Utilities|Casting|CastToAIControllerDailyLife_BP NewController))
  (bind _returnvalue (Rendering|Material|CreateDynamicMaterialInstance (Variables|Character|GetMesh) 0 0 "None" :!class /Script/Engine.PrimitiveComponent))
  (switch Utilities|FlowControl|Switch|SwitchonAIGuyTypes (Variables|/Game/Blueprints/AIControllerDailyLife_BP.AIControllerDailyLife_BP_C|GetAIGuyType _asaicontroller_daily_life_bp)
    (:NewEnumerator0
      (Rendering|Material|SetVectorParameterValue _returnvalue "Colour" "(R=1.000000,G=1.000000,B=0.000000,A=1.000000)" :!class /Script/Engine.MaterialInstanceDynamic))
    (:NewEnumerator1
      (Rendering|Material|SetVectorParameterValue _returnvalue "Colour" "(R=1.000000,G=0.000000,B=0.000000,A=1.000000)" :!class /Script/Engine.MaterialInstanceDynamic))
    (:NewEnumerator2
      (Rendering|Material|SetVectorParameterValue _returnvalue "Colour" "(R=0.000000,G=0.000000,B=1.000000,A=1.000000)" :!class /Script/Engine.MaterialInstanceDynamic))))

(event EventUseObject
  (params (UsedObject :type Actor%20Object%20Reference)))

(event EventUsed
  (params (UsingActor :type Actor%20Object%20Reference) (Value :type Integer))
  (bind _output_get (Variables|Default|SetInnerValue (+ Value (Variables|Default|GetInnerValue)))) ; We set some generic value of this object
  (Variables|Default|SetIsUsable false)
  (Rendering|Components|TextRender|SetText (Variables|Default|GetTextRender) (Utilities|Text|ToText(Integer) _output_get))
  (if (== UsingActor (AI|GetAIController self))
    (CallFunction|UpdateTransformforSelfActivity)))

(event EventBeginPlay)

(fn ConstructionScript)

(fn UpdateTransformforSelfActivity
  (bind _newparam (Utilities|DeltaSelfSleepingTransform))
  (bind (_location _rotation) (Math|Transform|BreakTransform _newparam))
  (switch Utilities|FlowControl|Switch|SwitchonActivityState (Utilities|Enum|ByteToEnumActivityState (Class|BlackboardComponent|GetValueasEnum (AI|GetBlackboard (AI|GetAIController self)) (Variables|Default|GetActivityChosenKeyName)))
    (:NewEnumerator10
      (if (Variables|Default|GetIsUsable)
        (Transformation|AddActorLocalRotation (Class|KismetMathLibrary|NegateRotator _rotation) false false)
        (Transformation|AddActorLocalOffset (* _location -1.0) false false)
        (else
          (Class|Actor|AddActorLocalTransform _newparam false false))))))

(fn CanbeUsed
  (params (UsingActor :type Actor%20Object%20Reference))
  (return (Variables|Default|GetIsUsable)))