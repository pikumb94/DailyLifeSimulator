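; Ping pong table that daily-life AI characters can use until MaxUsers is reached, with group use and joining disabled.
; Use snaps the AI pawn to a player socket chosen by user count; reset detaches it and frees the slot.
; When usable, it starts an empty-callback timer randomized by LonePreference, writing remaining time to each user's BlackboardTime so later joiners share the countdown.
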(event Custom|CustomEvent_0)

(event EventResetUsage
  (params (ResetInvokerActor :type Actor%20Object%20Reference))
  (Variables|Default|SetCurrentUsers (- (Variables|Default|GetCurrentUsers) 1))
  (Variables|Default|SetIsUsable true)
  (bind _asaicontroller_daily_life_bp (Utilities|Casting|CastToAIControllerDailyLife_BP ResetInvokerActor))
  (bind _asaiguy (Utilities|Casting|CastToAIGuy (Pawn|GetControlledPawn _asaicontroller_daily_life_bp)))
  (Transformation|DetachFromActor _asaiguy "KeepWorld" "KeepWorld" "KeepWorld"))

(event EventUsed
  (params (UsingActor :type Actor%20Object%20Reference) (Value :type Integer))
  (bind _staticmesh (Variables|Default|GetStaticMesh))
  (Variables|Default|SetCurrentUsers (+ (Variables|Default|GetCurrentUsers) 1))
  (bind _asaicontroller_daily_life_bp (Utilities|Casting|CastToAIControllerDailyLife_BP UsingActor))
  (bind _asaiguy (Utilities|Casting|CastToAIGuy (Pawn|GetControlledPawn _asaicontroller_daily_life_bp)))
  (if (Variables|Default|GetIsUsable)
    (bind _returnvalue (Utilities|Time|SetTimerbyEvent (delegate Custom|CustomEvent_0) (+ (* (Math|Random|RandomFloatinRange (- 1.0 (Variables|/Game/Blueprints/AIGuy.AIGuy_C|GetLonePreference _asaiguy)) 1.0) 3e+01) 3e+01))))
  (Variables|Default|SetIsUsable false)
  (AI|Components|Blackboard|SetValueasFloat (AI|GetBlackboard _asaicontroller_daily_life_bp) (Utilities|Name|MakeLiteralName "BlackboardTime") (Utilities|Time|GetTimerRemainingTimebyHandle _returnvalue))
  (if (== (Variables|Default|GetCurrentUsers) 1)
    (Transformation|AttachComponentToComponent (Pawn|GetControlledPawn _asaicontroller_daily_life_bp) _staticmesh "P1Socket" "SnapToTarget" "SnapToTarget" "KeepWorld" false)
    (else
      (Transformation|AttachComponentToComponent (Pawn|GetControlledPawn _asaicontroller_daily_life_bp) _staticmesh "P2Socket" "SnapToTarget" "SnapToTarget" "KeepWorld" false))))

(fn ConstructionScript)

(fn CanbeGroupJoined
  (params (UsingActor :type Actor%20Object%20Reference))
  (return false))

(fn CanbeGroupUsed
  (params (UsingActor :type Actor%20Object%20Reference))
  (return false))

(fn CanbeUsed
  (params (UsingActor :type Actor%20Object%20Reference))
  (if (>= (Variables|Default|GetCurrentUsers) (Variables|Default|GetMaxUsers))
    (return false)
    (else
      (return true))))